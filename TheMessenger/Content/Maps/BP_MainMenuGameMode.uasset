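; Game mode for the main menu that sets up the menu's input and UI when play begins.
; On BeginPlay it switches the first player controller to UI-only input without mouse lock, shows the cursor and adds a BPW_ widget to the viewport.
; Disconnected nodes for a cinematic intro widget, a dialogue HUD and fullscreen mode never run.
; Tick and the construction script are empty.
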(event `self.ReceiveBeginPlay`
  (bind _returnvalue (`GameplayStatics.GetPlayerController` 0))
  (`WidgetBlueprintLibrary.SetInputMode_UIOnlyEx` _returnvalue null)
  (set `PlayerController.bShowMouseCursor` true _returnvalue)
  (bind _returnvalue_2 (`|CreateWidget` "/Game/Blueprints/Widgets/Menus/EndScreen/BPW_.BPW__C" _returnvalue))
  (`UserWidget.AddToViewport` _returnvalue_2 0))

(fn `UserConstructionScript`)