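; BP_Building_1_2 is a medieval village building whose windows change to a warm yellow when the level starts at night.
; The construction script gathers its window glass mesh components into a Windows array.
; On BeginPlay it finds the LevelManager and, if the time type is Night, sets the "color" vector parameter on each window's materials.
; The time is checked only once, with no handling for other time types.
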(event `self.ReceiveBeginPlay`
  (bind _returnvalue (`GameplayStatics.GetActorOfClass` "/Script/TheMessenger.LevelManager"))
  (bind _output_get (set `self.LevelManager` _returnvalue))
  (switch `ETimeType` (`LevelManager.GetCurrentTimeType` _output_get)
    (:`Night`
      (for _array_element (`self.Windows`)
        (`MeshComponent.SetVectorParameterValueOnMaterials` _array_element "color" (0.5 0.5 0.1))))))

(fn `UserConstructionScript`
  (set `self.Windows` (`|MakeArray` (`self.SM_window_glass_81_StaticMeshComponent0`) (`self.SM_window_glass_13_StaticMeshComponent0`) (`self.SM_window_glass_14_StaticMeshComponent0`) (`self.SM_window_glass_15_StaticMeshComponent0`) (`self.SM_window_glass_75_StaticMeshComponent0`) (`self.SM_window_glass_76_StaticMeshComponent0`) (`self.SM_window_glass_79_StaticMeshComponent0`) (`self.SM_window_glass_80_StaticMeshComponent0`) (`self.SM_window_glass_12_StaticMeshComponent0`) (`self.SM_window_glass_82_StaticMeshComponent0`) (`self.SM_window_glass_98_StaticMeshComponent0`))))