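; BP_FollowingCharacter is an AI character that follows the player once its FollowPlayer event is triggered.
; BeginPlay caches the player as a TheMessengerCharacter reference.
; FollowPlayer moves toward the player when they are at least a set distance away, and otherwise targets itself to hold position.
; The event re-runs itself on a short delay after issuing each move, forming a polling loop that this graph never starts.
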(event `self.ReceiveBeginPlay`
  (bind _asthe_messenger_character (cast `TheMessengerCharacter` (`GameplayStatics.GetPlayerCharacter` 0)))
  (set `self.PlayerReference` _asthe_messenger_character))

(event `self.FollowPlayer`
  (if (>= (`self.GetDistanceTo` (`self.PlayerReference`)) 400.0)
    (`|AIMoveTo` self (0.0 0.0 0.0) (`self.PlayerReference`)
      (:`then`
        _))
    (else
      (`|AIMoveTo` self (0.0 0.0 0.0) self
        (:`then`
          _))))
  (`KismetSystemLibrary.Delay` 0.2)
  (`self.FollowPlayer`))

(fn `UserConstructionScript`)