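; BP_Burning_Villager is a building-related actor that keeps a villager hidden until it receives an impact event.
; On BeginPlay it hides itself, disables collision, and hides the Villager_Base taken from its BPVillagerBase2 child actor.
; OnImpactActor reverses this, showing the actor, re-enabling collision and revealing the villager.
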(event `self.ReceiveBeginPlay`
  (`self.SetActorHiddenInGame` true)
  (`self.SetActorEnableCollision` false)
  (bind _asvillager_base (cast `Villager_Base` (`ChildActorComponent.ChildActor` (`self.BP_Villager_Base_2`))))
  (bind _output_get (set `self.Villager_Base` _asvillager_base))
  (`Villager_Base.HideCharacter` _output_get true))

(event `self.OnImpactActor`
  (`self.SetActorHiddenInGame` false)
  (`self.SetActorEnableCollision` true)
  (`Villager_Base.HideCharacter` (`self.Villager_Base`) false))

(fn `UserConstructionScript`)